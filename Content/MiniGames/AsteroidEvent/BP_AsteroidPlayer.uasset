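; BP_AsteroidPlayer is the player for the asteroid event minigame, with sideways strafing and a placeholder shoot action.
; BeginPlay moves it to a fixed start location below the world origin.
; The Strafe axis adds movement along the control rotation's right vector only while its Y position is within symmetric bounds, so input in either direction stops outside them.
; Shoot only prints a message; no projectile logic exists.
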(event `self.ReceiveBeginPlay`
  (`self.K2_SetActorLocation` (0.0 0.0 -1500.0)))

(event `InputAction|Shoot`
  (params (Key :type "Key Structure"))
  (:`Pressed`
    (`KismetSystemLibrary.PrintString` "Pew Pew!")))

(event `InputAxis|Strafe`
  (params (AxisValue :type "Float (single-precision)"))
  (bind (_returnvalue_x _returnvalue_y) (`KismetMathLibrary.BreakVector` (`self.K2_GetActorLocation`)))
  (if (and (>= _returnvalue_y -1600.0) (<= _returnvalue_y 1600.0))
    (`self.AddMovementInput` (`KismetMathLibrary.GetRightVector` (`self.GetControlRotation`)) AxisValue)))

(fn `UserConstructionScript`)