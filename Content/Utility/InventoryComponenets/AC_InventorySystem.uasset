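; AC_InventorySystem is an actor component that handles world interaction and opens the inventory widget.
; Every tick it sphere-traces from the camera along its forward vector, caches the hit actor as LookAtActor and prints its look-at message when the target changes.
; The Interact input sends an interact message to that actor, and the Inventory input creates a new WBP_Inventory on each press.
; AddToInventory and RemoveFromInventory are empty stubs.
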(event `self.ReceiveTick`
  (params (DeltaSeconds :type "Float (single-precision)"))
  (`self.InteractionTrace`))

(event `InputAction|Inventory`
  (params (Key :type "Key Structure"))
  (:`Pressed`
    (bind _returnvalue (`|CreateWidget` "/Game/Utility/Widgets/WBP_Inventory.WBP_Inventory_C"))
    (`UserWidget.AddToViewport` _returnvalue 0)))

(event `InputAction|Interact`
  (params (Key :type "Key Structure"))
  (:`Pressed`
    (bind _lookatactor (`self.LookAtActor`)
      (:`then`
        (message `/Game/Utility/InventoryComponenets/BI_InteractInterface.InteractWith` _lookatactor))
      (:`else`))))

(fn `AddToInventory`)

(fn `InteractionTrace`
  (bind _returnvalue (`GameplayStatics.GetPlayerCameraManager` 0))
  (bind _returnvalue_2 (`Actor.K2_GetActorLocation` _returnvalue))
  (bind (_outhit _returnvalue_3) (`KismetSystemLibrary.SphereTraceSingle` _returnvalue_2 (+ _returnvalue_2 (* (`Actor.GetActorForwardVector` _returnvalue) (`self.InteractionRange`))) 15.0 "TraceTypeQuery3" false (`|MakeArray` (`self.GetOwner`))))
  (if _returnvalue_3
    (bind (_bblockinghit _binitialoverlap _time _distance _location _impactpoint _normal _impactnormal _physmat _hitactor) (`GameplayStatics.BreakHitResult` _outhit))
    (if (!= _hitactor (`self.LookAtActor`))
      (bind _output_get (set `self.LookAtActor` _hitactor))
      (bind _message (message `/Game/Utility/InventoryComponenets/BI_InteractInterface.LookAt` _output_get))
      (`KismetSystemLibrary.PrintString` (`KismetTextLibrary.Conv_TextToString` _message)))
    (else
      (set `self.LookAtActor` null))))

(fn `RemoveFromInventory`)